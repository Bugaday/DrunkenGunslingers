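; BP_CharMain is a player character Blueprint that moves by physics and shows a world-space cursor under the mouse.
; Forward and right axis inputs apply acceleration-based forces to the box collider along its own axes, scaled by MovementForce.
; Each tick, a cursor trace places CursorToWorld at the hit point, aligned to the surface normal.
; A physical animation setup for simulating skeletal bodies below a bone is present but unconnected.
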(event `self.ReceiveBeginPlay`)

(event `self.ReceiveTick`
  (params (DeltaSeconds :type "Float (single-precision)"))
  (bind (_bblockinghit _binitialoverlap _time _distance _location _impactpoint _normal _impactnormal) (`GameplayStatics.BreakHitResult` (`PlayerController.GetHitResultUnderCursorByChannel` (`GameplayStatics.GetPlayerController` 0) "TraceTypeQuery1" true)))
  ;[1 1 1] Set cursor to mouse position
  (`SceneComponent.K2_SetWorldLocationAndRotation` (`self.CursorToWorld`) _location (`KismetMathLibrary.MakeRotationFromAxes` _impactnormal) false false))

(event `InputAxis|MoveForward`
  (params (AxisValue :type "Float (single-precision)"))
  (bind _boxcollider (`self.BoxCollider`))
  (`PrimitiveComponent.AddForce` _boxcollider (* (`SceneComponent.GetForwardVector` _boxcollider) (* AxisValue (`self.MovementForce`))) "None" true))

(event `InputAxis|MoveRight`
  (params (AxisValue :type "Float (single-precision)"))
  (bind _boxcollider (`self.BoxCollider`))
  (`PrimitiveComponent.AddForce` _boxcollider (* (`SceneComponent.GetRightVector` _boxcollider) (* AxisValue (`self.MovementForce`))) "None" true))

(fn `UserConstructionScript`)