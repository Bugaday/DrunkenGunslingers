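; BP_Bullet is a projectile that moves along its forward vector every Tick at BulletSpeed, without sweeping.
; It stretches TrailRoot's Y scale by a clamped 2D distance between SpawnLocation and its position.
; SpawnLocation holds the per-frame movement delta, so that distance effectively measures from world origin rather than the firing point.
; Capsule overlaps only print the other actor's name, with no damage or destruction.
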(event `self.ReceiveTick`
  (params (DeltaSeconds :type "Float (single-precision)"))
  (bind _output_get (set `self.SpawnLocation` (* (`self.GetActorForwardVector`) (* (`self.BulletSpeed`) (`GameplayStatics.GetWorldDeltaSeconds`)))))
  (bind _sweephitresult (`self.K2_AddActorWorldOffset` _output_get))
  (bind _output_get_2 (set `self.TrailScaleY` (`KismetMathLibrary.FClamp` (/ (`KismetMathLibrary.Vector_Distance2D` (`self.SpawnLocation`) (`self.K2_GetActorLocation`)) 400.0) 0.0 1.0)))
  (`SceneComponent.SetRelativeScale3D` (`self.TrailRoot`) (`KismetMathLibrary.MakeVector` 3.0 _output_get_2 1.0))
  (`SceneComponent.SetRelativeScale3D` (`self.TrailRoot`) (`KismetMathLibrary.MakeVector` 3.0 _output_get_2 1.0)))

(event `self.Capsule.OnComponentBeginOverlap`
  (params (OverlappedComponent :type "PrimitiveComponent Object Reference") (OtherActor :type "Actor Object Reference") (OtherComp :type "PrimitiveComponent Object Reference") (OtherBodyIndex :type Integer) (bFromSweep :type Boolean) (SweepResult :type "HitResult Structure (by ref)"))
  (`KismetSystemLibrary.PrintString` (`KismetSystemLibrary.GetDisplayName` OtherActor)))

(fn `UserConstructionScript`)